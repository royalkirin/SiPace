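; Actor component that gives its owning Character a grappling hook, driven by a Ready, Firing and Attached state.
; FireGrapple launches a projectile hook with an attached cable actor toward a target.
; On hit it launches the character, suspends gravity and ground friction, then pulls every tick until the character nears or passes the hook, detected by a 2D dot product.
; Destroying the hook removes the cable and restores fixed movement values.
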(event `self.ReceiveTick`
  (params (DeltaSeconds :type "Float (single-precision)"))
  (switch `/Game/BluePrints/GrappleHook/Enum_Grapple` (`self.GrappleState`)
    (:`NewEnumerator2`
      (bind _ascharacter (cast `Character` (`self.GetOwner`)))
      (`CharacterMovementComponent.AddForce` (`Character.CharacterMovement` _ascharacter) (* (`self.GrappleDirection`) (`self.GrapplePullForce`)))
      (if (< (`KismetMathLibrary.Vector_Distance` (`Actor.K2_GetActorLocation` (`self.Grapple`)) (`Actor.K2_GetActorLocation` (`self.GetOwner`))) (`self.GrappleDestroyDistance`))
        (`Actor.K2_DestroyActor` (`self.Grapple`) :!label _label)
        (elif (< (`KismetMathLibrary.Dot_VectorVector` (`self.InitialHookDirection`) (`self.GrappleDirection2D`)) 0.0)
          (goto _label))))))

(fn `CancelGrapple`
  (bind _grapple (`self.Grapple`)
    (:`then`
      (`Actor.K2_DestroyActor` _grapple))
    (:`else`)))

(fn `FireGrapple`
  (params (Target :type "Vector Structure") (LocalOffset :type "Vector Structure"))
  (locals (FireDirection :type "Vector Structure" :default (0.0 0.0 0.0)))
  (bind _firedirection (`local.FireDirection`))
  (bind _returnvalue (`self.CableStartLocation` (`local.LocalOffset`)))
  (bind _cablecomponent (`CableActor.CableComponent` (`self.GrappleCable`)))
  ;[1 1 1] Check & Switch to Fire Mode
  (if (not (`self.InUse?`))
    (set `self.GrappleState` "NewEnumerator1")
    ;[1 1 1] Check & Spawn Grapple
    (set `local.FireDirection` (`KismetMathLibrary.Normal` (- (`local.Target`) _returnvalue)))
    (bind _returnvalue_2 (`|SpawnActorFromClass` "/Game/BluePrints/GrappleHook/Actor_Grapple.Actor_Grapple_C" (`KismetMathLibrary.MakeTransform` _returnvalue) "Undefined" "OverrideRootScale" null (* _firedirection (`self.GrappleSpeed`)) 3000.0 null))
    (bind _output_get (set `self.Grapple` _returnvalue_2))
    (add `Actor.OnActorHit` _output_get (`|CreateDelegate` :!event `GrappleHit`))
    (add `Actor.OnDestroyed` _output_get (`|CreateDelegate` :!event `GrappleDestroyed`))
    (bind _returnvalue_3 (`|SpawnActorFromClass` "/Game/BluePrints/GrappleHook/BP_GrappleCable.BP_GrappleCable_C" (`KismetMathLibrary.MakeTransform` _returnvalue (`KismetMathLibrary.MakeRotFromX` _firedirection)) "Undefined" "OverrideRootScale" null null))
    (bind _output_get_2 (set `self.GrappleCable` _returnvalue_3))
    (`Actor.K2_AttachToActor` _output_get_2 (`self.GetOwner`) "None" "KeepWorld" "KeepWorld" "KeepWorld" true)
    (`CableComponent.SetAttachEndTo` _cablecomponent (`self.Grapple`) "None" "None")
    (set `CableComponent.EndLocation` (0.0 0.0 0.0) _cablecomponent)))

(fn `GrappleDestroyed`
  (params (DestroyedActor :type "Actor Object Reference"))
  (set `self.Grapple` null)
  (set `self.GrappleState` "NewEnumerator0")
  (`|ExecutionSequence`
    (:`then_0`
      (bind _grapplecable (`self.GrappleCable`)
        (:`then`
          (`Actor.K2_DestroyActor` _grapplecable)
          (set `self.GrappleCable` null))
        (:`else`)))
    (:`then_1`
      ;[1 1 1] Reset Character On Ground Variables
      (bind _ascharacter (cast `Character` (`self.GetOwner`)))
      (bind _charactermovement (`Character.CharacterMovement` _ascharacter))
      (set `CharacterMovementComponent.GroundFriction` 1.0 _charactermovement)
      (set `CharacterMovementComponent.GravityScale` 1.75 _charactermovement)
      (set `CharacterMovementComponent.AirControl` 0.05 _charactermovement))))

(fn `GrappleHit`
  (params (SelfActor :type "Actor Object Reference") (OtherActor :type "Actor Object Reference") (NormalImpulse :type "Vector Structure") (Hit :type "HitResult Structure (by ref)"))
  (set `self.GrappleState` "NewEnumerator2")
  ;[1 1 1] Set Character On Air Variables
  (bind _ascharacter (cast `Character` (`self.GetOwner`)))
  (bind _charactermovement (`Character.CharacterMovement` _ascharacter))
  (set `CharacterMovementComponent.GroundFriction` 0.0 _charactermovement)
  (set `CharacterMovementComponent.GravityScale` 0.0 _charactermovement)
  (set `CharacterMovementComponent.AirControl` 0.2 _charactermovement)
  ;[1 1 1] Initial Pull Character
  (set `MovementComponent.Velocity` (* (`self.GrappleDirection`) (`self.GrapplnitialForce`)) _charactermovement)
  (set `self.InitialHookDirection` (`self.GrappleDirection2D`)))

(fn `InUse?`
  (returns (Result :type Boolean))
  (return (select `/Game/BluePrints/GrappleHook/Enum_Grapple` (`self.GrappleState`) :`NewEnumerator1` true :`NewEnumerator2` true)))