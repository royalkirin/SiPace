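; Grapple hook projectile actor that flies out when fired and cancels itself if it travels too far.
; On BeginPlay it applies its Velocity variable to the ProjectileMovement component and records its start location.
; Every tick it measures the distance from that start point and destroys itself once MaxDistance is reached.
; The graph contains no hit, attach or pull logic.
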(event `self.ReceiveBeginPlay`
  ;[1 1 1] Shoot Grapple
  (set `MovementComponent.Velocity` (`self.Velocity`) (`self.ProjectileMovement`))
  (set `self.StartLocation` (`self.K2_GetActorLocation`)))

(event `self.ReceiveTick`
  (params (DeltaSeconds :type "Float (single-precision)"))
  ;[1 1 1] Cancel Grapple: Too Long
  (if (>= (`KismetMathLibrary.Vector_Distance` (`self.StartLocation`) (`self.K2_GetActorLocation`)) (`self.MaxDistance`))
    (`self.K2_DestroyActor`)))

(fn `UserConstructionScript`)